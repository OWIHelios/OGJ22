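; BP_ToggleButton is a button actor that alternates between pressed and released each time its Toggle event is called, through a FlipFlop.
; Pressing sends SignalIndex through BPEventSender, plays a click sound and runs the ButtonDown timeline to lower the mesh.
; Releasing removes the signal and reverses the timeline, but only while no actors overlap the button.
; The FlipFlop still advances when a release is blocked.
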(event `Toggle`
  (bind _bp_eventsender (`self.BP_EventSender`))
  (bind _signalindex (`self.SignalIndex`))
  (`/Engine/EditorBlueprintResources/StandardMacros.FlipFlop`
    (:`A`
      (if (not (`self.IsTriggered`))
        (set `self.IsTriggered` true)
        (`/Game/Blueprints/EventSystem/BP_EventSender.SendSignal` _bp_eventsender _signalindex)
        (`GameplayStatics.PlaySoundAtLocation` "/Engine/VREditor/Sounds/UI/Click_on_Button.Click_on_Button" (`self.K2_GetActorLocation`) (struct) 1.0 1.0 0.0 null null null null)
        (bind (_direction _buttonmovement) (`Timeline|ButtonDown` :`NewTime` (`self.ButtonMoveTime`) :!label _label)
          (:`Update`
            (`SceneComponent.K2_SetRelativeLocation` (`self.StaticMesh1`) (`KismetMathLibrary.MakeVector` 0.0 0.0 (`KismetMathLibrary.Lerp` 0.0 (`self.ButtonDownOffset`) _buttonmovement)) false false)))))
    (:`B`
      (if (and (== (`KismetArrayLibrary.Array_Length` (`self.GetOverlappingActors` "/Script/Engine.Actor")) 0) (`self.IsTriggered`))
        (`/Game/Blueprints/EventSystem/BP_EventSender.RemoveSignal` _bp_eventsender _signalindex)
        (set `self.IsTriggered` false)
        (goto _label :!via `Reverse`)))))

(fn `UserConstructionScript`)