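; Player controller that drives the possessed BP_PlayerCharacter and handles the pause menu.
; Mouse axes turn the view with inverted pitch input, while movement axes follow the character camera's forward and right vectors, alongside a jump action.
; Escape press shows W_PauseMenu with UI-only input and a cursor.
; Escape release or the menu's resume event removes it and any options widget, restoring game-only input.
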(event `self.ReceiveBeginPlay`)

(event `self.ReceivePossess`
  (params (PossessedPawn :type "Pawn Object Reference"))
  (bind _asbp_player_character (cast `/Game/Blueprints/Core/BP_PlayerCharacter` PossessedPawn))
  (set `self.PlayerCharacter` _asbp_player_character))

(event `InputAxisKey|MouseX`
  (params (AxisValue :type "Float (single-precision)"))
  ;[1 1 1] Mouse Inputs
  (`self.AddYawInput` AxisValue))

(event `InputAxisKey|MouseY`
  (params (AxisValue :type "Float (single-precision)"))
  ;[1 1 1] Mouse Inputs
  (`self.AddPitchInput` (* AxisValue -1.0)))

(event `InputAxis|MoveForward`
  (params (AxisValue :type "Float (single-precision)"))
  (bind _playercharacter (`self.PlayerCharacter`))
  ;[1 1 1] Keyboard Inputs
  (`/Engine/EditorBlueprintResources/StandardMacros.IsValid` _playercharacter
    (:`Is Valid`
      (`Pawn.AddMovementInput` (`self.PlayerCharacter`) (`SceneComponent.GetForwardVector` (`/Game/Blueprints/Core/BP_PlayerCharacter.Camera` _playercharacter)) AxisValue false))))

(event `InputAxis|MoveRight`
  (params (AxisValue :type "Float (single-precision)"))
  (bind _playercharacter (`self.PlayerCharacter`))
  ;[1 1 1] Keyboard Inputs
  (`/Engine/EditorBlueprintResources/StandardMacros.IsValid` _playercharacter
    (:`Is Valid`
      (`Pawn.AddMovementInput` (`self.PlayerCharacter`) (`SceneComponent.GetRightVector` (`/Game/Blueprints/Core/BP_PlayerCharacter.Camera` _playercharacter)) AxisValue false))))

(event `InputAction|Jump`
  (params (Key :type "Key Structure"))
  ;[1 1 1] Keyboard Inputs
  (:`Pressed`
    (`/Engine/EditorBlueprintResources/StandardMacros.IsValid` (`self.PlayerCharacter`)
      (:`Is Valid`
        (`Character.Jump` (`self.PlayerCharacter`))))))

(event `Key|Escape`
  (params (Key :type "Key Structure"))
  (:`Pressed`
    (bind _returnvalue (`|CreateWidget` "/Game/Widgets/W_PauseMenu.W_PauseMenu_C"))
    (bind _output_get (set `self.PauseMenu` _returnvalue))
    (`UserWidget.AddToViewport` _returnvalue 0)
    (`WidgetBlueprintLibrary.SetInputMode_UIOnlyEx` self _output_get "LockOnCapture")
    (add `/Game/Widgets/W_PauseMenu.OnResume` _returnvalue (delegate `OnResume`))
    (set `self.bShowMouseCursor` true))
  (:`Released`
    (`self.OnResume`)))

(event `OnResume`
  (bind _pausemenu (`self.PauseMenu`))
  (bind _options (`/Game/Widgets/W_PauseMenu.Options` _pausemenu))
  (`/Engine/EditorBlueprintResources/StandardMacros.IsValid` _options
    (:`Is Valid`
      (`Widget.RemoveFromParent` _options))
    (:`Is Not Valid`
      _))
  (`Widget.RemoveFromParent` _pausemenu)
  (`WidgetBlueprintLibrary.SetInputMode_GameOnly` self)
  (set `self.bShowMouseCursor` false))

(fn `UserConstructionScript`
  (`WidgetBlueprintLibrary.SetInputMode_GameOnly` self))