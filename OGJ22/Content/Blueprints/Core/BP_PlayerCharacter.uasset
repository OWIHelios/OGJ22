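; BP_PlayerCharacter is the player character, handling mouse input for grabbing, releasing and throwing objects.
; On possession it sets player 0's controller to game-only input.
; Left press and release call TryGrab and TryRelease on BPPickupSystem, and right press calls TryThrow.
; Grab and throw presses play a sound at the character's location whether or not the attempt succeeds.
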(event `self.ReceivePossessed`
  (params (NewController :type "Controller Object Reference"))
  (`WidgetBlueprintLibrary.SetInputMode_GameOnly` (`GameplayStatics.GetPlayerController` 0)))

(event `Key|LeftMouseButton`
  (params (Key :type "Key Structure"))
  (bind _bp_pickupsystem (`self.BP_PickupSystem`))
  (:`Pressed`
    (`/Game/Blueprints/Pickup/BP_PickupSystem.TryGrab` _bp_pickupsystem)
    (`GameplayStatics.PlaySoundAtLocation` "/Engine/VREditor/Sounds/UI/Object_PickUp.Object_PickUp" (`self.K2_GetActorLocation`) (struct) 1.0 1.0 0.0 null null null null))
  (:`Released`
    (`/Game/Blueprints/Pickup/BP_PickupSystem.TryRelease` _bp_pickupsystem)))

(event `Key|RightMouseButton`
  (params (Key :type "Key Structure"))
  (:`Pressed`
    (`/Game/Blueprints/Pickup/BP_PickupSystem.TryThrow` (`self.BP_PickupSystem`))
    (`GameplayStatics.PlaySoundAtLocation` "/Engine/VREditor/Sounds/UI/Scaling_Down.Scaling_Down" (`self.K2_GetActorLocation`) (struct) 1.0 1.0 0.0 null null null null)))

(fn `UserConstructionScript`)