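; BP_EventSender is the sending half of an event system, passing indexed signals to a list of connected objects.
; SendSignal and RemoveSignal each loop over Connections, find the BP_EventReceiver component on every valid entry, and call OnReceivedEvent or RemoveSignalEvent on it.
; Invalid entries and those without a receiver component are skipped, and only the first receiver found on each entry is notified.
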(fn `RemoveSignal`
  (params (Signal :type Integer))
  (for _array_element (`self.Connections`)
    (`/Engine/EditorBlueprintResources/StandardMacros.IsValid` _array_element
      (:`Is Valid`
        (bind _returnvalue (`Actor.GetComponentByClass` _array_element "/Game/Blueprints/EventSystem/BP_EventReceiver.BP_EventReceiver_C"))
        (`/Engine/EditorBlueprintResources/StandardMacros.IsValid` _returnvalue
          (:`Is Valid`
            (`/Game/Blueprints/EventSystem/BP_EventReceiver.RemoveSignal_Event` _returnvalue (`local.Signal`))))))))

(fn `SendSignal`
  (params (Index :type Integer))
  (for _array_element (`self.Connections`)
    (`/Engine/EditorBlueprintResources/StandardMacros.IsValid` _array_element
      (:`Is Valid`
        (bind _returnvalue (`Actor.GetComponentByClass` _array_element "/Game/Blueprints/EventSystem/BP_EventReceiver.BP_EventReceiver_C"))
        (`/Engine/EditorBlueprintResources/StandardMacros.IsValid` _returnvalue
          (:`Is Valid`
            (`/Game/Blueprints/EventSystem/BP_EventReceiver.OnReceived_Event` _returnvalue (`local.Index`))))))))