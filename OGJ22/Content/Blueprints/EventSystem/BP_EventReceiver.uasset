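; BP_EventReceiver is an event-system Blueprint that counts received signals and reports when any count reaches TriggerAmount.
; OnReceived_Event increments the signal's entry in the CurrentTriggered map and calls CallOnReceived with that signal.
; RemoveSignal_Event stores key 0's decremented, clamped count under the given signal and passes that count to CallOnReceived.
; IsConditionMet scans the map and returns the first qualifying entry's array index, not its key, or -1.
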(event `RemoveSignal_Event`
  (params (Signal :type Integer))
  (bind _currenttriggered (`self.CurrentTriggered`))
  (bind _returnvalue (- (`BlueprintMapLibrary.Map_Find` _currenttriggered) 1))
  (bind _returnvalue_2 (`KismetMathLibrary.Clamp` _returnvalue 0 _returnvalue))
  (`BlueprintMapLibrary.Map_Add` _currenttriggered Signal _returnvalue_2)
  (`self.OnReceived` _returnvalue_2))

(event `OnReceived_Event`
  (params (SignalIndex :type Integer))
  (bind _currenttriggered (`self.CurrentTriggered`))
  (`BlueprintMapLibrary.Map_Add` _currenttriggered SignalIndex (+ (`BlueprintMapLibrary.Map_Find` _currenttriggered SignalIndex) 1))
  (`self.OnReceived` SignalIndex))

(fn `IsConditionMet`
  (returns (ConditionMet :type Boolean) (TriggerSignal :type Integer))
  (locals (LTrigAmount :type Integer))
  (bind _currenttriggered (`self.CurrentTriggered`))
  (bind _keys (`BlueprintMapLibrary.Map_Keys` _currenttriggered))
  (for (_array_element _array_index) _keys
    (if (>= (`BlueprintMapLibrary.Map_Find` _currenttriggered _array_element) (`self.TriggerAmount`))
      (return true _array_index)))
  (return false -1))