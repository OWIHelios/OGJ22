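; BP_Button is a pressure plate that sends an indexed signal through its BPEventSender while something overlaps its box trigger.
; The first overlap sets a triggered flag, sends the signal, plays a click sound and runs a timeline that lerps the button mesh down by an offset.
; When no overlapping actors remain, it removes the signal, clears the flag and reverses the timeline to raise the mesh.
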(event `self.Box.OnComponentBeginOverlap`
  (params (OverlappedComponent :type "PrimitiveComponent Object Reference") (OtherActor :type "Actor Object Reference") (OtherComp :type "PrimitiveComponent Object Reference") (OtherBodyIndex :type Integer) (bFromSweep :type Boolean) (SweepResult :type "HitResult Structure (by ref)"))
  (if (not (`self.IsTriggered`))
    (set `self.IsTriggered` true)
    (`/Game/Blueprints/EventSystem/BP_EventSender.SendSignal` (`self.BP_EventSender`) (`self.SignalIndex`))
    (`GameplayStatics.PlaySoundAtLocation` "/Engine/VREditor/Sounds/UI/Click_on_Button.Click_on_Button" (`self.K2_GetActorLocation`) (struct) 1.0 1.0 0.0 null null null null)
    (bind (_direction _buttonmovement) (`Timeline|ButtonDown` :`NewTime` (`self.ButtonMoveTime`) :!label _label)
      (:`Update`
        (`SceneComponent.K2_SetRelativeLocation` (`self.StaticMesh1`) (`KismetMathLibrary.MakeVector` 0.0 0.0 (`KismetMathLibrary.Lerp` 0.0 (`self.ButtonDownOffset`) _buttonmovement)) false false)))))

(event `self.Box.OnComponentEndOverlap`
  (params (OverlappedComponent :type "PrimitiveComponent Object Reference") (OtherActor :type "Actor Object Reference") (OtherComp :type "PrimitiveComponent Object Reference") (OtherBodyIndex :type Integer))
  (if (and (== (`KismetArrayLibrary.Array_Length` (`self.GetOverlappingActors` "/Script/Engine.Actor")) 0) (`self.IsTriggered`))
    (`/Game/Blueprints/EventSystem/BP_EventSender.RemoveSignal` (`self.BP_EventSender`) (`self.SignalIndex`))
    (set `self.IsTriggered` false)
    (goto _label :!via `Reverse`)))

(fn `UserConstructionScript`)