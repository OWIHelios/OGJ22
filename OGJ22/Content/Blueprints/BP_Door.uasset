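; BP_Door is a door that opens and closes in response to signals from its BP_EventReceiver component.
; When the receiver's condition is met with trigger signal 0, the OpenDoor timeline plays, lerping the Cube's relative Z toward ZOffset, and a sound plays at the door.
; When the condition is not met, the timeline reverses to move the Cube back, without triggering the sound.
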(event `self.BP_EventReceiver.OnReceived`
  (params (SignalIndex :type Integer))
  (bind _cube (`self.Cube`))
  (bind (_conditionmet _triggersignal) (`/Game/Blueprints/EventSystem/BP_EventReceiver.IsConditionMet` (`self.BP_EventReceiver`)))
  (bind (_relativelocation_x _relativelocation_y) (`KismetMathLibrary.BreakVector` (`SceneComponent.RelativeLocation` _cube)))
  (if _conditionmet
    (switch `int` _triggersignal
      (:`0`
        (`|ExecutionSequence`
          (:`then_0`
            (bind (_direction _newtrack_0) (`Timeline|OpenDoor` :!label _label)
              (:`Update`
                (`SceneComponent.K2_SetRelativeLocation` _cube (`KismetMathLibrary.MakeVector` _relativelocation_x _relativelocation_y (`KismetMathLibrary.Lerp` 0.0 (`self.ZOffset`) _newtrack_0)) false false))))
          (:`then_1`
            (`GameplayStatics.PlaySoundAtLocation` "/Engine/VREditor/Sounds/UI/Dockable_Window_Open.Dockable_Window_Open" (`self.K2_GetActorLocation`) (struct) 1.0 1.0 0.0 null null null null)))))
    (else
      (goto _label :!via `Reverse`))))

(fn `UserConstructionScript`)