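; Scene-based pickup system that lets its owner grab, carry, release and throw physical objects, and toggle buttons.
; TryGrab line-traces forward, grabbing actors tagged Pickable with collision and physics disabled, or toggling BP_ToggleButton actors tagged Interactable.
; Tick holds the grabbed actor at a fixed distance ahead, matching only the facing yaw.
; TryRelease restores collision and physics, while TryThrow also adds a forward impulse.
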(event `self.ReceiveTick`
  (params (DeltaSeconds :type "Float (single-precision)"))
  (bind _returnvalue (`self.GetForwardVector`))
  (bind _grabbingobject (`self.GrabbingObject`))
  (bind (_returnvalue_roll _returnvalue_pitch _returnvalue_yaw) (`KismetMathLibrary.BreakRotator` (`KismetMathLibrary.Conv_VectorToRotator` _returnvalue)))
  (if (`self.isGrabbing`)
    (`/Engine/EditorBlueprintResources/StandardMacros.IsValid` (`self.GrabbingObject`)
      (:`Is Valid`
        (`Actor.K2_SetActorLocation` _grabbingobject (+ (`self.K2_GetComponentLocation`) (* _returnvalue (`self.HoldDistance`))) false false)
        (`Actor.K2_SetActorRotation` _grabbingobject (`KismetMathLibrary.MakeRotator` 0.0 0.0 _returnvalue_yaw) false)))))

(event `TryGrab`
  (bind _returnvalue (`self.K2_GetComponentLocation`))
  (bind _outhit (`KismetSystemLibrary.LineTraceSingle` :`Start` _returnvalue :`End` (+ _returnvalue (* (`self.GetForwardVector`) (`self.TraceDist`))) :`TraceChannel` "TraceTypeQuery1" :`DrawDebugType` "ForDuration" :`DrawTime` 1.0))
  (bind _output_get (set `self.LastHitResult` _outhit))
  (bind (_bblockinghit _binitialoverlap _time _distance _location _impactpoint _normal _impactnormal _physmat _hitactor) (`GameplayStatics.BreakHitResult` _output_get))
  (`/Engine/EditorBlueprintResources/StandardMacros.IsValid` _hitactor
    (:`Is Valid`
      (if (`Actor.ActorHasTag` _hitactor "Pickable")
        (bind _output_get_2 (set `self.GrabbingObject` _hitactor))
        (`Actor.SetActorEnableCollision` _output_get_2 false)
        (bind _returnvalue_2 (`Actor.GetComponentByClass` _output_get_2 "/Script/Engine.PrimitiveComponent"))
        (`/Engine/EditorBlueprintResources/StandardMacros.IsValid` _returnvalue_2
          (:`Is Valid`
            (`PrimitiveComponent.SetSimulatePhysics` _returnvalue_2 false)
            (set `self.isGrabbing` true)))
        (elif (`Actor.ActorHasTag` _hitactor "Interactable")
          (bind _asbp_toggle_button (cast `/Game/Blueprints/BP_ToggleButton` _hitactor))
          (`/Game/Blueprints/BP_ToggleButton.Toggle` _asbp_toggle_button))))))

(event `TryRelease`
  (bind _grabbingobject (`self.GrabbingObject`))
  (bind _returnvalue (`Actor.GetComponentByClass` _grabbingobject "/Script/Engine.PrimitiveComponent"))
  (`/Engine/EditorBlueprintResources/StandardMacros.IsValid` (`self.GrabbingObject`)
    (:`Is Valid`
      (`Actor.SetActorEnableCollision` _grabbingobject true)
      (`/Engine/EditorBlueprintResources/StandardMacros.IsValid` _returnvalue
        (:`Is Valid`
          (`PrimitiveComponent.SetSimulatePhysics` _returnvalue true))
        (:`Is Not Valid`
          _))
      (set `self.GrabbingObject` null)
      (set `self.isGrabbing` false))))

(event `TryThrow`
  (bind _grabbingobject (`self.GrabbingObject`))
  (bind _returnvalue (`Actor.GetComponentByClass` _grabbingobject "/Script/Engine.PrimitiveComponent"))
  (`/Engine/EditorBlueprintResources/StandardMacros.IsValid` (`self.GrabbingObject`)
    (:`Is Valid`
      (`Actor.SetActorEnableCollision` _grabbingobject true)
      (set `self.isGrabbing` false)
      (`/Engine/EditorBlueprintResources/StandardMacros.IsValid` _returnvalue
        (:`Is Valid`
          (`PrimitiveComponent.SetSimulatePhysics` _returnvalue true)
          (`PrimitiveComponent.AddImpulse` _returnvalue (* (`self.GetForwardVector`) (`self.ThrowForce`)) "None" false))
        (:`Is Not Valid`
          _))
      (set `self.GrabbingObject` null))))