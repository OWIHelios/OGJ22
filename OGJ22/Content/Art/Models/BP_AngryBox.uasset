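; BP_AngryBox is a physics box actor with an icon screen that can return to its starting transform.
; The construction script creates a dynamic CoreScreen material, sets its image from StatesIcons by IconIndex and applies it to the mesh's second slot.
; BeginPlay caches the mesh's world transform.
; TriggerReset starts a ResetTimer delay, after which Reset teleports the actor back and clears physics velocities.
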(event `self.ReceiveBeginPlay`
  (bind _staticmeshcomponent (`self.StaticMeshComponent`))
  (set `self.OriginalLocation` (`SceneComponent.K2_GetComponentLocation` _staticmeshcomponent))
  (set `self.OriginalOrientation` (`SceneComponent.K2_GetComponentRotation` _staticmeshcomponent)))

(event `TriggerReset`
  (`KismetSystemLibrary.K2_SetTimerDelegate` (delegate `Reset`) (`self.ResetTimer`)))

(event `Reset`
  (bind _staticmeshcomponent (`self.StaticMeshComponent`))
  (`self.K2_SetActorLocation` (`self.OriginalLocation`) false true)
  (`self.K2_SetActorRotation` (`self.OriginalOrientation`))
  (`PrimitiveComponent.SetAllPhysicsLinearVelocity` _staticmeshcomponent (0.0 0.0 0.0) false)
  (`PrimitiveComponent.SetAllPhysicsAngularVelocityInDegrees` _staticmeshcomponent (0.0 0.0 0.0) false))

(fn `UserConstructionScript`
  (bind _output (`|GetArrayItem` (`self.StatesIcons`) (`self.IconIndex`)))
  (bind _returnvalue (`KismetMaterialLibrary.CreateDynamicMaterialInstance` "/Game/Art/Models/CoreScreen.CoreScreen"))
  (`/Engine/EditorBlueprintResources/StandardMacros.IsValid` _output
    (:`Is Valid`
      (`MaterialInstanceDynamic.SetTextureParameterValue` _returnvalue "Image" _output)
      (`PrimitiveComponent.SetMaterial` (`self.StaticMeshComponent`) 1 _returnvalue))))